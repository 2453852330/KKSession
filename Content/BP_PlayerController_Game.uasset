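; Player controller that handles leaving a multiplayer session and server-initiated map travel through debug-style F and G keys.
; F destroys the session via KKSessionSubsystem, then opens Map_Example regardless of the result.
; On success, the server calls the ROC destroy event on every controller of this class, which destroys that session and returns to Map_Example.
; G, server only, issues a ServerTravel console command targeting Map_TravelTo.
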(event Custom|OnDestorySesisonFinish
  (params (bSuccess :type Boolean))
  (Game|OpenLevel(byObjectReference) "/KKSession/Map_Example.Map_Example")
  (if bSuccess
    (if (or (Networking|IsServer) (Networking|IsDedicatedServer))
      (bind _outactors (Actor|GetAllActorsOfClass "BP_PlayerController_Game_C"))
      (for _array_element _outactors
        (CallFunction|ROCDestorySession _array_element)))
    (else
      (Development|PrintString "destory session failed"))))

(event Custom|ROC_DestorySession
  (Class|KKSessionSubsystem|KKDestorySession (Subsystems|GetKKSessionSubsystem) self (delegate Custom|CustomEvent_0)))

(event Custom|CustomEvent_0
  (params (bSuccess :type Boolean))
  (if bSuccess
    (Game|OpenLevel(byObjectReference) "/KKSession/Map_Example.Map_Example")
    (else
      (Development|PrintString "roc destory sesison failed"))))

(event Input|KeyboardEvents|F
  (params (Key :type Key%20Structure :default "None"))
  (:Pressed
    (Class|KKSessionSubsystem|KKDestorySession (Subsystems|GetKKSessionSubsystem) self (delegate Custom|OnDestorySesisonFinish))))

(event Input|KeyboardEvents|G
  (params (Key :type Key%20Structure :default "None"))
  (:Pressed
    (if (or (Networking|IsServer) (Networking|IsDedicatedServer))
      (Development|PrintString "Travel")
      (Development|ExecuteConsoleCommand (Utilities|String|Append "ServerTravel " "Map_TravelTo") self))))

(fn ConstructionScript)